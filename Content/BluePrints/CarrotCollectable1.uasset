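; Carrot pickup Blueprint that the third-person character collects by entering its sphere trigger.
; On overlap it plays a collect sound at the world origin and starts the Attraction timeline, which lerps the carrot from its current location toward the character's live position.
; When the timeline finishes, it calls CollectCarrot on the character and destroys itself.
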(event OnComponentBeginOverlap(Sphere)
  (params (OverlappedComponent :type Primitive%20Component%20Object%20Reference) (OtherActor :type Actor%20Object%20Reference) (OtherComp :type Primitive%20Component%20Object%20Reference) (OtherBodyIndex :type Integer) (bFromSweep :type Boolean) (SweepResult :type Hit%20Result%20Structure%20%28by%20ref%29))
  (bind _asthird_person_character (Utilities|Casting|CastToThirdPersonCharacter OtherActor))
  (Audio|PlaySoundatLocation "/Game/FreeSounds/CarrotCollect.CarrotCollect" "0, 0, 0" "0, 0, 0" 1.0 1.0 0.0 0 0 0)
  (bind _distance (Timeline|Attraction Play)
    (:Update
      (Transformation|SetWorldLocation (Variables|Default|GetCarrot) (Math|Vector|Lerp(Vector) (Transformation|GetWorldLocation (Variables|Default|GetCarrot)) (Transformation|GetActorLocation _asthird_person_character) _distance) false false))
    (:Finished
      (Default|CollectCarrot _asthird_person_character)
      (Actor|DestroyActor))))

(fn ConstructionScript)