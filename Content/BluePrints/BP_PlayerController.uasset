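; BP_PlayerController is a player controller Blueprint that handles the player's death and game restart.
; Its OnDeath event unpossesses the pawn, starts a held camera fade and shows a DeadScreen widget.
; After a short delay it removes the widget and calls RestartGame on the ThirdPersonGameMode.
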(event Custom|OnDeath
  (Pawn|UnPossess)
  (CameraFades|StartCameraFade :self (Variables|Default|GetPlayerCameraManager) :ToAlpha 1.0 :Duration 1.0 :bHoldWhenFinished true)
  (bind _returnvalue (UserInterface|CreateWidget "/Game/UI/DeadScreen.DeadScreen_C" self))
  (UserInterface|Viewport|AddtoViewport _returnvalue 0)
  (Utilities|FlowControl|Delay 2.0)
  (Widget|RemovefromParent _returnvalue)
  (bind _asthird_person_game_mode (Utilities|Casting|CastToThirdPersonGameMode (Game|GetGameMode)))
  (Class|GameMode|RestartGame _asthird_person_game_mode))

(event EventBeginPlay)

(event EventTick
  (params (DeltaSeconds :type Float%20%28single-precision%29)))

(fn ConstructionScript)